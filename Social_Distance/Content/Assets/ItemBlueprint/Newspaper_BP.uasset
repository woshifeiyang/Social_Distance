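; Clickable newspaper item that advances a quest task when the player picks it up.
; GlowToggle or the 2 key flips a highlight using custom depth and a dynamic material's Alpha parameter.
; A click within range while task 0 is at its required stage triggers the character's picking animation and a Niagara effect.
; Input is UI-only during a timed delay, then returns to Game and UI as the task advances.
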(event `self.ReceiveBeginPlay`
  (bind _returnvalue (`PrimitiveComponent.CreateDynamicMaterialInstance` (`self.Newspaper`) 0 "/Game/Assets/material/newspaper.newspaper" "None"))
  (`self.EnableInput` (`GameplayStatics.GetPlayerController` 0)))

(event `GlowToggle`
  (bind _newspaper (`self.Newspaper`))
  (`/Engine/EditorBlueprintResources/StandardMacros.FlipFlop` :!label _label
    (:`A`
      (`PrimitiveComponent.SetRenderCustomDepth` _newspaper true)
      (`MaterialInstanceDynamic.SetScalarParameterValue` (stale `self.ReceiveBeginPlay` _returnvalue) "Alpha" 1.0))
    (:`B`
      (`PrimitiveComponent.SetRenderCustomDepth` _newspaper false)
      (`MaterialInstanceDynamic.SetScalarParameterValue` (stale `self.ReceiveBeginPlay` _returnvalue) "Alpha" 0.0))))

(event `Key|Two`
  (params (Key :type "Key Structure"))
  (:`Pressed`
    (goto _label)))

(event `self.Newspaper.OnClicked`
  (params (TouchedComponent :type "PrimitiveComponent Object Reference") (ButtonPressed :type "Key Structure"))
  (bind _returnvalue (`GameplayStatics.GetPlayerController` 0))
  (bind _maincharacter (`self.MainCharacter`))
  (bind (_value _returnvalue_2) (`BlueprintMapLibrary.Map_Find` (`MainCharacter.TaskList` _maincharacter)))
  (bind _returnvalue_3 (`GameplayStatics.GetActorOfClass` "/Game/ThirdPersonCPP/Blueprints/MyMainCharacter.MyMainCharacter_C"))
  (bind _asmy_main_character (cast `/Game/ThirdPersonCPP/Blueprints/MyMainCharacter` _returnvalue_3))
  (bind _output_get (set `self.MainCharacter` _asmy_main_character))
  (if (and _returnvalue_2 (<= (`KismetMathLibrary.Vector_Distance` (`MainCharacter.SelfLocation` _maincharacter) (`self.K2_GetActorLocation` self)) 200.0) (== _value 1))
    (bind _asmain_character_anim_instance (cast `MainCharacterAnimInstance` (`SkeletalMeshComponent.GetAnimInstance` (`Character.Mesh` _output_get))))
    (bind _output_get_2 (set `self.As Main Character Anim Instance` _asmain_character_anim_instance))
    (set `MainCharacterAnimInstance.IsPicking` true _output_get_2)
    (`AddComponent|NODE_AddNiagaraComponent-0` :`self` (`self.MainCharacter`) :`RelativeTransform` (`KismetMathLibrary.MakeTransform` (`KismetMathLibrary.MakeVector` 0.0 0.0 (+ 0.0 150.0)) (struct) (3.0 3.0 3.0)))
    (`WidgetBlueprintLibrary.SetInputMode_UIOnlyEx` _returnvalue null)
    (`KismetSystemLibrary.Delay` 4.0)
    (`WidgetBlueprintLibrary.SetInputMode_GameAndUIEx` _returnvalue null)
    (set `MainCharacterAnimInstance.IsPicking` false (`self.As Main Character Anim Instance`))
    (`BlueprintMapLibrary.Map_Add` (`MainCharacter.TaskList` (`self.MainCharacter`)) 0 2)))

(fn `UserConstructionScript`)