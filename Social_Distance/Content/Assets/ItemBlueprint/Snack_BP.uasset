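; Snack item actor with three baguette meshes that the player clicks to complete a stage of task 2.
; A one-second looping timer polls the main character's TaskList and, while that task is at stage 1, highlights the meshes through custom depth and a dynamic material Alpha.
; Clicking within range at that stage triggers the picking animation and a Niagara effect, switches input to UI-only during a delay, then advances the task to stage 2.
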(event `self.ReceiveBeginPlay`
  ;[1 1 1] Item glowwing
  (bind _returnvalue (`GameplayStatics.GetActorOfClass` "/Game/ThirdPersonCPP/Blueprints/MyMainCharacter.MyMainCharacter_C"))
  (bind _asmy_main_character (cast `/Game/ThirdPersonCPP/Blueprints/MyMainCharacter` _returnvalue))
  (set `self.As My Main Character` _asmy_main_character)
  (`KismetSystemLibrary.K2_SetTimerDelegate` (delegate `Check`) 1.0 true)
  (bind _returnvalue_2 (`PrimitiveComponent.CreateDynamicMaterialInstance` (`self.baguette`) 0 "/Game/Assets/material/Mid-tone1.Mid-tone1" "None"))
  (bind _returnvalue_3 (`PrimitiveComponent.CreateDynamicMaterialInstance` (`self.baguette1`) 0 "/Game/Assets/material/Mid-tone1.Mid-tone1" "None"))
  (bind _returnvalue_4 (`PrimitiveComponent.CreateDynamicMaterialInstance` (`self.baguette2`) 0 "/Game/Assets/material/Mid-tone1.Mid-tone1" "None"))
  (`self.EnableInput` (`GameplayStatics.GetPlayerController` 0)))

(event `Check`
  (bind _baguette2 (`self.baguette2`))
  (bind _as_my_main_character (`self.As My Main Character`))
  (bind _baguette (`self.baguette`))
  (bind _baguette1 (`self.baguette1`))
  (bind (_value _returnvalue) (`BlueprintMapLibrary.Map_Find` (`MainCharacter.TaskList` _as_my_main_character) 2))
  ;[1 1 1] Item glowwing
  (if (`KismetSystemLibrary.IsValid` _as_my_main_character)
    (if (and _returnvalue (== _value 1))
      (`PrimitiveComponent.SetRenderCustomDepth` _baguette true)
      (`MaterialInstanceDynamic.SetScalarParameterValue` (stale `self.ReceiveBeginPlay` _returnvalue_2) "Alpha" 1.0)
      (`PrimitiveComponent.SetRenderCustomDepth` _baguette1 true)
      (`MaterialInstanceDynamic.SetScalarParameterValue` (stale `self.ReceiveBeginPlay` _returnvalue_2) "Alpha" 1.0)
      (`MaterialInstanceDynamic.SetScalarParameterValue` (stale `self.ReceiveBeginPlay` _returnvalue_3) "Alpha" 1.0)
      (`PrimitiveComponent.SetRenderCustomDepth` _baguette2 true)
      (`MaterialInstanceDynamic.SetScalarParameterValue` (stale `self.ReceiveBeginPlay` _returnvalue_4) "Alpha" 1.0)
      (else
        (`PrimitiveComponent.SetRenderCustomDepth` _baguette false)
        (`MaterialInstanceDynamic.SetScalarParameterValue` (stale `self.ReceiveBeginPlay` _returnvalue_2) "Alpha" 0.0)
        (`PrimitiveComponent.SetRenderCustomDepth` _baguette1 false)
        (`MaterialInstanceDynamic.SetScalarParameterValue` (stale `self.ReceiveBeginPlay` _returnvalue_3) "Alpha" 0.0)
        (`PrimitiveComponent.SetRenderCustomDepth` _baguette2 false)
        (`MaterialInstanceDynamic.SetScalarParameterValue` (stale `self.ReceiveBeginPlay` _returnvalue_4) "Alpha" 0.0)))))

(event `self.ReceiveActorOnClicked`
  (params (ButtonPressed :type "Key Structure"))
  (bind _returnvalue (`GameplayStatics.GetPlayerController` 0))
  (bind _as_my_main_character (`self.As My Main Character`))
  (bind (_value _returnvalue_2) (`BlueprintMapLibrary.Map_Find` (`MainCharacter.TaskList` _as_my_main_character) 2))
  (if (and _returnvalue_2 (<= (`KismetMathLibrary.Vector_Distance` (`MainCharacter.SelfLocation` _as_my_main_character) (`self.K2_GetActorLocation` self)) 200.0) (== _value 1))
    (bind _asmain_character_anim_instance (cast `MainCharacterAnimInstance` (`SkeletalMeshComponent.GetAnimInstance` (`Character.Mesh` (`self.As My Main Character`)))))
    (bind _output_get (set `self.As Main Character Anim Instance` _asmain_character_anim_instance))
    (set `MainCharacterAnimInstance.IsPicking` true _output_get)
    (`AddComponent|NODE_AddNiagaraComponent-0` :`self` (`self.As My Main Character`) :`RelativeTransform` (`KismetMathLibrary.MakeTransform` (`KismetMathLibrary.MakeVector` 0.0 0.0 (+ 0.0 150.0)) (struct) (3.0 3.0 3.0)))
    (`WidgetBlueprintLibrary.SetInputMode_UIOnlyEx` _returnvalue null)
    (`KismetSystemLibrary.Delay` 4.0)
    (`WidgetBlueprintLibrary.SetInputMode_GameAndUIEx` _returnvalue null)
    (set `MainCharacterAnimInstance.IsPicking` false (`self.As Main Character Anim Instance`))
    (`BlueprintMapLibrary.Map_Add` (`MainCharacter.TaskList` (`self.As My Main Character`)) 2 2)))

(fn `UserConstructionScript`)